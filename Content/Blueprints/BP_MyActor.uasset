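; Actor that drives a cutout material on a plane using textures built at runtime from TIFF channels.
; BeginPlay creates the dynamic material, and ShowHole1 turns extracted channel 3 into its DynamicTexture.
; A FadeOut timeline animates Fade Amount, while RemoveT2DArrayChannel updates the material's texture array and Size.
; Alpha2 and Alpha3 only extract channels; fade-in, bulk channel generation and array-adding logic are disconnected.
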(event `self.ReceiveBeginPlay`
  (bind _plane (`self.Plane`))
  (`|ExecutionSequence`
    (:`then_0`
      ;[0 0.01442 1] Set a dynamic material instance
      (bind _returnvalue (`KismetMaterialLibrary.CreateDynamicMaterialInstance` (`PrimitiveComponent.GetMaterial` _plane 0)))
      (bind _output_get (set `self.DM_CutoutMaterial` _returnvalue))
      (`PrimitiveComponent.SetMaterial` _plane 0 _output_get)
      (`MaterialInstanceDynamic.SetScalarParameterValue` _output_get "None" 0.0))))

(event `self.ReceiveTick`
  (params (DeltaSeconds :type "Float (single-precision)")))

(event `ShowHole1`
  (bind (_imagewidth _imageheight _returnvalue) (`self.ExtractTiffChannels` 3))
  (bind _returnvalue_2 (`self.CreateTexture2DDynamicFromChannelData` _imagewidth _imageheight _returnvalue))
  (bind _output_get (set `self.NewVar_0` _returnvalue_2))
  (`MaterialInstanceDynamic.SetTextureParameterValue` (`self.DM_CutoutMaterial`) "DynamicTexture" _output_get))

(event `Alpha 2`
  (params (Index :type Integer :default 4) (Value :type "Float (single-precision)" :default 2.0))
  (`self.ExtractTiffChannels` Index))

(event `Fade Out`
  (bind (_direction _newtrack_0) (`Timeline|FadeOut` :!via `PlayFromStart`)
    (:`Update`
      (`MaterialInstanceDynamic.SetScalarParameterValue` (`self.DM_CutoutMaterial`) "Fade Amount" _newtrack_0))))

(event `Alpha 3`
  (params (Index :type Integer :default 5) (Value :type "Float (single-precision)" :default 3.0))
  (`self.ExtractTiffChannels` Index))

(fn `RemoveT2DArrayChannel`
  (params (Texture :type "Texture2D Object Reference (by ref)"))
  (bind _dm_cutoutmaterial (`self.DM_CutoutMaterial`))
  (bind (_size _returnvalue) (`self.UpdateTexture2DArray` Texture true))
  (`MaterialInstanceDynamic.SetTextureParameterValue` _dm_cutoutmaterial "Texture2DObject" _returnvalue)
  (`MaterialInstanceDynamic.SetScalarParameterValue` _dm_cutoutmaterial "Size" (`KismetMathLibrary.Conv_IntToDouble` _size))
  (return))

(fn `UserConstructionScript`)